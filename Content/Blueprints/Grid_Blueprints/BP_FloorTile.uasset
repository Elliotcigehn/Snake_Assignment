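; BP_FloorTile is a floor tile actor that positions itself as one cell of a grid.
; Initialize, when a valid owner exists, attaches the tile to that owner, snapping location and rotation while keeping relative scale.
; It then offsets itself by Row along X and Column along Y, using the FloorTile component's full bounds as cell size.
; The event graph and construction script are empty.
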(fn `Initialize`
  (bind _returnvalue (`self.GetOwner`))
  (`/Engine/EditorBlueprintResources/StandardMacros.IsValid` _returnvalue
    (:`Is Valid`
      (`self.K2_AttachToActor` _returnvalue "None" "SnapToTarget" "SnapToTarget" "KeepRelative" false)
      (`self.K2_SetActorRelativeLocation` (`KismetMathLibrary.MakeVector` (* (.x (* (`.BoxExtent` (`KismetSystemLibrary.GetComponentBounds` (`self.FloorTile`))) (2.0 2.0 0.0))) (`self.Row`)) (* (.y (* (`.BoxExtent` (`KismetSystemLibrary.GetComponentBounds` (`self.FloorTile`))) (2.0 2.0 0.0))) (`self.Column`)))))))

(fn `UserConstructionScript`)