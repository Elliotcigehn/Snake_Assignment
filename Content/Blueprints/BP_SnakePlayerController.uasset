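; Player controller for the snake game that scales difficulty with score and handles pausing.
; Every tick it looks up the BP_BoxRoverPawn and reads its Score, stepping its own MovementSpeed up and TurnSpeed down as score thresholds are passed.
; The G key toggles pause through a FlipFlop, creating or removing the pause widget, setting the game's paused state and showing or hiding the mouse cursor.
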(event `self.ReceiveTick`
  (params (DeltaSeconds :type "Float (single-precision)"))
  (bind _returnvalue (`GameplayStatics.GetActorOfClass` "/Game/Blueprints/BP_BoxRoverPawn.BP_BoxRoverPawn_C"))
  (bind _asbp_box_rover_pawn (cast `/Game/Blueprints/BP_BoxRoverPawn` _returnvalue))
  (if (> (`/Game/Blueprints/BP_BoxRoverPawn.Score` _asbp_box_rover_pawn) 90)
    (set `self.movementSpeed` 800.0)
    (set `self.turnSpeed` 110.0)
    (if (> (`/Game/Blueprints/BP_BoxRoverPawn.Score` _asbp_box_rover_pawn) 240)
      (set `self.movementSpeed` 1000.0)
      (set `self.turnSpeed` 100.0)
      (if (> (`/Game/Blueprints/BP_BoxRoverPawn.Score` _asbp_box_rover_pawn) 490)
        (set `self.movementSpeed` 1200.0)
        (set `self.turnSpeed` 90.0)))))

(event `Key|G` :paused true
  (params (Key :type "Key Structure"))
  (:`Pressed`
    (`/Engine/EditorBlueprintResources/StandardMacros.FlipFlop`
      (:`A`
        (bind _returnvalue (`|CreateWidget` (`self.PauseWidgetClass`)))
        (set `self.PauseWidget` _returnvalue)
        (`UserWidget.AddToViewport` (`self.PauseWidget`) 0)
        (`GameplayStatics.SetGamePaused` true)
        (set `self.bShowMouseCursor` true))
      (:`B`
        (`Widget.RemoveFromParent` (`self.PauseWidget`))
        (`GameplayStatics.SetGamePaused` false)
        (set `self.bShowMouseCursor` false)))))

(fn `UserConstructionScript`)