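; Teleporter actor that moves an overlapping snake pawn to an offset above and beside its TargetTeleporter.
; On box overlap, an IsSnake check gates the move, then a BP_BoxRoverPawn cast allows repositioning the instanced tail mesh relative to the pawn.
; Its own box and the tail drop collision, restored after a short delay only if the cast succeeds.
; IsTeleporter identifies the actor, while Teleported is an empty stub.
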(event `self.ReceiveActorBeginOverlap`
  (params (OtherActor :type "Actor Object Reference")))

(event `self.Box.OnComponentBeginOverlap`
  (params (OverlappedComponent :type "PrimitiveComponent Object Reference") (OtherActor :type "Actor Object Reference") (OtherComp :type "PrimitiveComponent Object Reference") (OtherBodyIndex :type Integer) (bFromSweep :type Boolean) (SweepResult :type "HitResult Structure (by ref)"))
  (bind _yes_no (message `/Game/Blueprints/BPI_Snake.IsSnake` OtherActor))
  (if _yes_no
    (`PrimitiveComponent.SetCollisionEnabled` (`self.Box`) "NoCollision")
    (`self.K2_SetActorLocation` OtherActor (+ (`self.K2_GetActorLocation` (`self.TargetTeleporter_`)) (100.0 0.0 200.0)) false false)
    (bind _asbp_box_rover_pawn (cast `/Game/Blueprints/BP_BoxRoverPawn` OtherActor))
    (bind _ism_snaketail (`/Game/Blueprints/BP_BoxRoverPawn.ISM_SnakeTail` _asbp_box_rover_pawn))
    (`PrimitiveComponent.SetCollisionEnabled` _ism_snaketail "NoCollision")
    (`SceneComponent.K2_SetWorldLocation` _ism_snaketail (- (`self.K2_GetActorLocation` OtherActor) (2000.0 0.0 -500.0)) false false)
    (`KismetSystemLibrary.Delay` 2.0)
    (`PrimitiveComponent.SetCollisionEnabled` (`self.Box`) "QueryOnly")
    (`PrimitiveComponent.SetCollisionEnabled` _ism_snaketail "ProbeOnly")))

(fn `IsTeleporter`
  (returns (`Yes/No` :type Boolean))
  (return true))

(fn `Teleported`
  (params (`Yes/No` :type Boolean))
  (returns (Snake :type "/Game/Blueprints/BP_BoxRoverPawn Object Reference"))
  (return null))

(fn `UserConstructionScript`)