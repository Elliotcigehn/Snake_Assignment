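; BP_Food is a food pickup actor that moves to a new spot when consumed instead of being destroyed.
; Its construction script finds and stores the MyGridGeneratorISM actor, which the Consume event calls to reposition the food on the NavMesh.
; Tick slowly spins the Sphere component by a fixed per-frame step, and IsFood always returns true to identify the actor as food.
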(event `self.ReceiveTick`
  (params (DeltaSeconds :type "Float (single-precision)"))
  (`SceneComponent.K2_AddRelativeRotation` (`self.Sphere`) (struct :`Yaw` 0.1) false false))

(event `/Game/Blueprints/BPI_Food.Consume`
  (`GridGeneratorISM.RePositionFoodOnNavMesh` (`self.GridRef`) self))

(fn `IsFood`
  (returns (`Yes/No` :type Boolean))
  (return true))

(fn `UserConstructionScript`
  (bind _returnvalue (`GameplayStatics.GetActorOfClass` "/Game/Blueprints/Grid_Blueprints/MyGridGeneratorISM.MyGridGeneratorISM_C"))
  (set `self.GridRef` _returnvalue))