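; BP_BoxRoverPawn is the player pawn of a Snake game, with a tail built from detached instanced static mesh segments.
; While moving, it pins the first instance to the actor and lerps each following one toward its predecessor's previous transform.
; Interface checks on overlap identify walls, which trigger game over through SnakeGameMode, and food, which adds score and a segment.
; Tail overlaps send Die to actors identifying as snake bodies.
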(event `self.ReceiveTick`
  (params (DeltaSeconds :type "Float (single-precision)"))
  (if (> (`KismetMathLibrary.VSize` (`self.GetVelocity`)) 0.0)
    (`self.LerpLocations`)))

(event `LerpLocations`
  (bind (_returnvalue_location _returnvalue_rotation) (`KismetMathLibrary.BreakTransform` (`self.GetTransform`)))
  (bind _ism_snaketail (`self.ISM_SnakeTail`))
  (bind (_output_location _output_rotation _output_scale) (`KismetMathLibrary.BreakTransform` (`|GetArrayItem` (`self.InstanceTransform`))))
  (`KismetArrayLibrary.Array_Clear` (`self.InstanceTransform`))
  (for _index (range (+ (- (`InstancedStaticMeshComponent.GetInstanceCount` (`self.ISM_SnakeTail`)) 0) 1))
    (`KismetArrayLibrary.Array_Add` (`self.InstanceTransform`) (`InstancedStaticMeshComponent.GetInstanceTransform` (`self.ISM_SnakeTail`) _index true)))
  (`InstancedStaticMeshComponent.UpdateInstanceTransform` (`self.ISM_SnakeTail`) 0 (`KismetMathLibrary.MakeTransform` _returnvalue_location _returnvalue_rotation _output_scale) true false false)
  (for (_array_element _array_index) (`self.InstanceTransform`)
    (bind _returnvalue (+ _array_index 1))
    (`InstancedStaticMeshComponent.UpdateInstanceTransform` _ism_snaketail _returnvalue (`KismetMathLibrary.TLerp` (`InstancedStaticMeshComponent.GetInstanceTransform` _ism_snaketail _returnvalue true) _array_element 0.05) true false false)))

(event `self.Collision.OnComponentBeginOverlap`
  (params (OverlappedComponent :type "PrimitiveComponent Object Reference") (OtherActor :type "Actor Object Reference") (OtherComp :type "PrimitiveComponent Object Reference") (OtherBodyIndex :type Integer) (bFromSweep :type Boolean) (SweepResult :type "HitResult Structure (by ref)"))
  (bind _ism_snaketail (`self.ISM_SnakeTail`))
  (bind _yes_no (message `/Game/Blueprints/Grid_Blueprints/BPI_GridGenerator.IsWall` OtherActor))
  (if _yes_no
    (`/Game/Blueprints/BPI_SnakeCollisionWithSelf.Die`)
    (else
      (bind _yes_no_2 (message `/Game/Blueprints/BPI_Food.IsFood` OtherActor))
      (if _yes_no_2
        (message `/Game/Blueprints/BPI_Food.Consume` OtherActor)
        (set `self.Score` (+ (`self.Score`) 10))
        (`InstancedStaticMeshComponent.AddInstance` _ism_snaketail (`InstancedStaticMeshComponent.GetInstanceTransform` _ism_snaketail (- (`InstancedStaticMeshComponent.GetInstanceCount` _ism_snaketail) 1) true) true)))))

(event `self.ISM_SnakeTail.OnComponentBeginOverlap`
  (params (OverlappedComponent :type "PrimitiveComponent Object Reference") (OtherActor :type "Actor Object Reference") (OtherComp :type "PrimitiveComponent Object Reference") (OtherBodyIndex :type Integer) (bFromSweep :type Boolean) (SweepResult :type "HitResult Structure (by ref)"))
  (bind _yes_no (message `/Game/Blueprints/BPI_SnakeCollisionWithSelf.IsSnakeBody` OtherActor))
  (if _yes_no
    (message `/Game/Blueprints/BPI_SnakeCollisionWithSelf.Die` OtherActor)))

(event `/Game/Blueprints/BPI_SnakeCollisionWithSelf.Die`
  (bind _returnvalue (`GameplayStatics.GetActorOfClass` "/Script/Snake_Assignment.SnakeGameMode"))
  (`SnakeGameMode.TriggerGameOver` _returnvalue))

(fn `IsSnake`
  (returns (`Yes/No` :type Boolean))
  (return true))

(fn `IsSnakeBody`
  (returns (`Yes/No` :type Boolean) (SnakeBody :type "Vector Structure"))
  (return true (`self.Instance Transform Scale`)))

(fn `UserConstructionScript`
  (bind _ism_snaketail (`self.ISM_SnakeTail`))
  (`SceneComponent.K2_DetachFromComponent` _ism_snaketail "KeepWorld" "KeepWorld" "KeepWorld" true)
  (`InstancedStaticMeshComponent.ClearInstances` _ism_snaketail)
  (for _index (range (+ (`self.BodyAmount`) 1))
    (`InstancedStaticMeshComponent.AddInstance` (`self.ISM_SnakeTail`) (`KismetMathLibrary.MakeTransform` (`KismetMathLibrary.MakeVector` (`KismetMathLibrary.Conv_IntToDouble` (* _index (`self.Spacing`)))) (struct) (`self.Instance Transform Scale`)) false)))